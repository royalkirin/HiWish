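; Player pawn that moves sideways within fixed Y bounds, with a dash, a power jump and health that pauses into a death screen at zero.
; Dash boosts speed and raises side guards while draining its meter in a per-tick delay loop.
; Jump uses a timeline for height and arrow-key lateral motion, with top guards raised.
; SaveGame and LoadGame persist player stats, score and BP_Spawner tuning through SaveStats, loading on BeginPlay.
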(event EventBeginPlay
  (bind _outactors (Actor|GetAllActorsOfClass "/Game/BluePrints/Enemy/BP_Spawner.BP_Spawner_C"))
  (Variables|Default|SetSpawnerREF (Utilities|Array|Get(acopy) _outactors))
  (CallFunction|LoadGame (Variables|Default|GetSavedSlotName))
  (Variables|Default|SetHealth (Variables|Default|GetMaxHealth))
  (Variables|Default|SetDashMeter (Variables|Default|GetDashMax)))

(event Collision|EventActorBeginOverlap
  (params (OtherActor :type Actor%20Object%20Reference)))

(event Game|Damage|EventAnyDamage
  (params (Damage :type Float%20%28single-precision%29) (DamageType :type Damage%20Type%20Object%20Reference) (InstigatedBy :type Controller%20Object%20Reference) (DamageCauser :type Actor%20Object%20Reference))
  ;[1 1 1] Taking Damage
  (Variables|Default|SetHealth (- (Variables|Default|GetHealth) Damage))
  (if (> (Variables|Default|GetHealth) 0.0)
    (Development|PrintString "Ouch")
    (else
      (bind _returnvalue (UserInterface|CreateWidget "/Game/UI_HUD/DeathHUD.DeathHUD_C"))
      (UserInterface|Viewport|AddtoViewport _returnvalue 0)
      (Game|SetGamePaused true)
      (Variables|/Script/Engine.PlayerController|SetbShowMouseCursor (Game|GetPlayerController 0) true))))

(event Input|ActionEvents|InputActionDash
  (params (Key :type Key%20Structure :default "None"))
  (bind _float (Variables|Default|GetFloat))
  (bind _float_2 (Variables|Default|GetFloat))
  ;[1 1 1] Dashing
  (:Pressed
    (Variables|Default|SetDashPressed true)
    (if (> (Variables|Default|GetDashMeter) 0.0)
      (Variables|Default|SetIsDashing true)
      (Variables|/Script/Engine.FloatingPawnMovement|SetMaxSpeed _float (* (Variables|/Script/Engine.FloatingPawnMovement|GetMaxSpeed _float) (Variables|Default|GetDashMultiple)))
      (CallFunction|SideGuardon)
      (Variables|Default|SetDashMeter (- (Variables|Default|GetDashMeter) (/ (Utilities|Time|GetWorldDeltaSeconds) 0.1)) :!label _label)
      (Utilities|FlowControl|DelayUntilNextTick)
      (if (and (> (Variables|Default|GetDashMeter) 0.0) (Variables|Default|GetDashPressed))
        (goto _label)
        (else
          (Variables|Default|SetIsDashing false)
          (Variables|/Script/Engine.FloatingPawnMovement|SetMaxSpeed _float_2 (/ (Variables|/Script/Engine.FloatingPawnMovement|GetMaxSpeed _float_2) (Variables|Default|GetDashMultiple)))
          (CallFunction|SideGuardOff)))))
  (:Released
    (Variables|Default|SetDashPressed false)
    (Variables|Default|SetIsDashing false)))

(event Input|ActionEvents|InputActionJump
  (params (Key :type Key%20Structure :default "None"))
  (bind _returnvalue (Transformation|GetActorLocation))
  (bind _returnvalue_2 (Game|GetPlayerController 0))
  ;[1 1 1] PowerJump
  (:Pressed
    (CallFunction|TopGuardon)
    (Variables|Default|SetIsJumping true)
    (bind (_direction _jumptrack _jumpy) (Timeline|JumpTimeline PlayFromStart)
      (:Update
        (if (Game|Player|IsInputKeyDown _returnvalue_2 "Left")
          (Variables|Default|SetJumpSpeed (* (Math|Float|Absolute(Float) (Variables|Default|GetJumpSpeed)) -1.0))
          (Transformation|SetActorLocation (Math|Vector|MakeVector (.x _returnvalue) (+ (.y _returnvalue) (Math|Float|Lerp 0.0 (Variables|Default|GetJumpSpeed) _jumpy)) (Math|Float|Lerp 0.0 3e+02 _jumptrack)) false false :!label _label)
          (elif (Game|Player|IsInputKeyDown _returnvalue_2 "Right")
            (Variables|Default|SetJumpSpeed (Math|Float|Absolute(Float) (Variables|Default|GetJumpSpeed)))
            (goto _label)
            (else
              (Transformation|SetActorLocation (Math|Vector|MakeVector (.x _returnvalue) (.y _returnvalue) (Math|Float|Lerp 0.0 3e+02 _jumptrack)) false false)))))
      (:Finished
        (Variables|Default|SetIsJumping false)
        (CallFunction|TopGuardOff)))))

(event Input|AxisEvents|InputAxisMoveRight/Left
  (params (AxisValue :type Float%20%28single-precision%29))
  (bind _returnvalue (Transformation|GetActorLocation))
  (bind _returnvalue_2 (Pawn|GetControlRotation :!class /Script/Engine.Pawn))
  (bind _returnvalue_3 (Math|Vector|GetRightVector (Math|Rotator|MakeRotator (.roll _returnvalue_2) 0.0 (.yaw _returnvalue_2))))
  ;[1 1 1] Left/Right Movement
  (if (> (.y _returnvalue) -1e+03)
    (if (< (.y _returnvalue) 1e+03)
      (Pawn|Input|AddMovementInput _returnvalue_3 AxisValue false)
      (else
        (Pawn|Input|AddMovementInput _returnvalue_3 (Math|Float|Clamp(Float) AxisValue -1.0 0.0) false)))
    (else
      (Pawn|Input|AddMovementInput _returnvalue_3 (Math|Float|Clamp(Float) AxisValue) false))))

(event Input|KeyboardEvents|1
  (params (Key :type Key%20Structure :default "None"))
  (:Pressed
    (Development|PrintString (Utilities|String|ToString(Float) (Variables|Default|GetJumpSpeed)))))

(fn ConstructionScript)

(fn SaveGame
  (params (SlotName :type String))
  (bind _spawnerref (Variables|Default|GetSpawnerREF))
  (bind _spawnerref_2 (Variables|Default|GetSpawnerREF))
  (bind _returnvalue (SaveGame|DoesSaveGameExist SlotName))
  (if _returnvalue
    (bind _returnvalue_2 (SaveGame|LoadGamefromSlot SlotName))
    (Variables|Default|SetSaveREF _returnvalue_2)
    (else
      (bind _returnvalue_3 (SaveGame|CreateSaveGameObject "/Game/SaveGame/SaveStats.SaveStats_C"))
      (bind _output_get (Variables|Default|SetSaveREF _returnvalue_3))))
  (bind _assave_stats (Utilities|Casting|CastToSaveStats _output_get))
  (Variables|/Game/SaveGame/SaveStats.SaveStats_C|SetMaxHealth _assave_stats (Variables|Default|GetMaxHealth))
  (Variables|/Game/SaveGame/SaveStats.SaveStats_C|SetDashMax _assave_stats (Variables|Default|GetDashMax))
  (Variables|/Game/SaveGame/SaveStats.SaveStats_C|SetGoodSpawnRate _assave_stats (Variables|/Game/BluePrints/Enemy/BP_Spawner.BP_Spawner_C|GetGoodSpawnRate _spawnerref))
  (Variables|/Game/SaveGame/SaveStats.SaveStats_C|SetSpawnRate _assave_stats (Variables|/Game/BluePrints/Enemy/BP_Spawner.BP_Spawner_C|GetSpawnRate _spawnerref))
  (Variables|/Game/SaveGame/SaveStats.SaveStats_C|SetDropSpeed _assave_stats (Variables|/Game/BluePrints/Enemy/BP_Spawner.BP_Spawner_C|GetDropSpeed _spawnerref))
  (Variables|/Game/SaveGame/SaveStats.SaveStats_C|SetDiamondRate _assave_stats (Variables|/Game/BluePrints/Enemy/BP_Spawner.BP_Spawner_C|GetDiamondSpawnRate _spawnerref_2))
  (Variables|/Game/SaveGame/SaveStats.SaveStats_C|SetPouchValue _assave_stats (Variables|/Game/BluePrints/Enemy/BP_Spawner.BP_Spawner_C|GetPouchValue _spawnerref_2))
  (Variables|/Game/SaveGame/SaveStats.SaveStats_C|SetMoney _assave_stats (Variables|Impose|GetScore))
  (Variables|/Game/SaveGame/SaveStats.SaveStats_C|SetDashSpeed _assave_stats (Variables|Default|GetDashMultiple))
  (Variables|/Game/SaveGame/SaveStats.SaveStats_C|SetLevel _assave_stats (Variables|Default|GetLevel))
  (Variables|/Game/SaveGame/SaveStats.SaveStats_C|SetUpgradeCount _assave_stats (Variables|Default|GetUpgradeCount))
  (Variables|/Game/SaveGame/SaveStats.SaveStats_C|SetJumpSpeed _assave_stats (Variables|Default|GetJumpSpeed))
  (SaveGame|SaveGametoSlot (Variables|Default|GetSaveREF) SlotName))

(fn LoadGame
  (params (SlotName :type String))
  (bind _spawnerref (Variables|Default|GetSpawnerREF))
  (bind _spawnerref_2 (Variables|Default|GetSpawnerREF))
  (bind _returnvalue (SaveGame|DoesSaveGameExist SlotName))
  (if _returnvalue
    (bind _returnvalue_2 (SaveGame|LoadGamefromSlot SlotName))
    (bind _assave_stats (Utilities|Casting|CastToSaveStats _returnvalue_2))
    (Variables|Default|SetMaxHealth (Variables|/Game/SaveGame/SaveStats.SaveStats_C|GetMaxHealth _assave_stats))
    (Variables|Default|SetDashMax (Variables|/Game/SaveGame/SaveStats.SaveStats_C|GetDashMax _assave_stats))
    (Variables|/Game/BluePrints/Enemy/BP_Spawner.BP_Spawner_C|SetGoodSpawnRate _spawnerref (Variables|/Game/SaveGame/SaveStats.SaveStats_C|GetGoodSpawnRate _assave_stats))
    (Variables|/Game/BluePrints/Enemy/BP_Spawner.BP_Spawner_C|SetSpawnRate _spawnerref (Variables|/Game/SaveGame/SaveStats.SaveStats_C|GetSpawnRate _assave_stats))
    (Variables|/Game/BluePrints/Enemy/BP_Spawner.BP_Spawner_C|SetDropSpeed _spawnerref (Variables|/Game/SaveGame/SaveStats.SaveStats_C|GetDropSpeed _assave_stats))
    (Variables|/Game/BluePrints/Enemy/BP_Spawner.BP_Spawner_C|SetDiamondSpawnRate _spawnerref_2 (Variables|/Game/SaveGame/SaveStats.SaveStats_C|GetDiamondRate _assave_stats))
    (Variables|/Game/BluePrints/Enemy/BP_Spawner.BP_Spawner_C|SetPouchValue _spawnerref_2 (Variables|/Game/SaveGame/SaveStats.SaveStats_C|GetPouchValue _assave_stats))
    (Variables|Impose|SetScore (Variables|/Game/SaveGame/SaveStats.SaveStats_C|GetMoney _assave_stats))
    (Variables|Default|SetDashMultiple (Variables|/Game/SaveGame/SaveStats.SaveStats_C|GetDashSpeed _assave_stats))
    (Variables|Default|SetLevel (Variables|/Game/SaveGame/SaveStats.SaveStats_C|GetLevel _assave_stats))
    (Variables|Default|SetUpgradeCount (Variables|/Game/SaveGame/SaveStats.SaveStats_C|GetUpgradeCount _assave_stats))
    (Variables|Default|SetJumpSpeed (Variables|/Game/SaveGame/SaveStats.SaveStats_C|GetJumpSpeed _assave_stats))))

(fn TopGuardon
  (bind _toprightguard (Variables|Default|GetTopRightGuard))
  (Rendering|SetVisibility _toprightguard true false)
  (Collision|SetCollisionProfileName _toprightguard "BlockBad" true :!class /Script/Engine.PrimitiveComponent))

(fn TopGuardOff
  (bind _toprightguard (Variables|Default|GetTopRightGuard))
  (Rendering|SetVisibility _toprightguard false false)
  (Collision|SetCollisionProfileName _toprightguard "NoCollision" true :!class /Script/Engine.PrimitiveComponent))

(fn SideGuardon
  (bind _leftguard (Variables|Default|GetLeftGuard))
  (Rendering|SetVisibility _leftguard true false)
  (Collision|SetCollisionProfileName _leftguard "BlockBad" true :!class /Script/Engine.PrimitiveComponent))

(fn SideGuardOff
  (bind _leftguard (Variables|Default|GetLeftGuard))
  (Rendering|SetVisibility _leftguard false false)
  (Collision|SetCollisionProfileName _leftguard "NoCollision" true :!class /Script/Engine.PrimitiveComponent))