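; BP_Gold is a short-lived gold pickup that adds its GoldValue to the player's Score.
; Overlapping its Collision component with a PlayerPawn awards the score and destroys the actor, while other actors are ignored.
; Uncollected gold destroys itself after a fixed delay from BeginPlay.
; Tick spins the mesh on all three axes, scaled by delta time for frame-rate independence.
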(event OnComponentBeginOverlap(Collision)
  (params (OverlappedComponent :type Primitive%20Component%20Object%20Reference) (OtherActor :type Actor%20Object%20Reference) (OtherComp :type Primitive%20Component%20Object%20Reference) (OtherBodyIndex :type Integer) (bFromSweep :type Boolean) (SweepResult :type Hit%20Result%20Structure%20%28by%20ref%29))
  ;[1 1 1] Calculate Score
  (bind _asplayer_pawn (Utilities|Casting|CastToPlayerPawn OtherActor))
  (Variables|/Game/BluePrints/Character/PlayerPawn.PlayerPawn_C|SetScore _asplayer_pawn (+ (Variables|/Game/BluePrints/Character/PlayerPawn.PlayerPawn_C|GetScore _asplayer_pawn) (Variables|Property|GetGoldValue)))
  (Actor|DestroyActor))

(event EventTick
  (params (DeltaSeconds :type Float%20%28single-precision%29))
  (bind _returnvalue (* DeltaSeconds 1.5e+02))
  ;[1 1 1] Spin
  (Transformation|AddLocalRotation (Variables|Default|GetMesh) (Math|Rotator|MakeRotator _returnvalue _returnvalue _returnvalue) false false))

(event EventBeginPlay
  (Utilities|FlowControl|Delay 5.0)
  (Actor|DestroyActor))

(fn ConstructionScript)