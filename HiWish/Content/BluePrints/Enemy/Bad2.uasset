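; Bad2 is an enemy Blueprint that spins a Geometry Collection on all three axes every tick and destroys itself five seconds after BeginPlay.
; Its hit and overlap events are empty.
; Disconnected logic would tell a player pawn hit from a guard, which turns on physics and disables collision.
; A separate unwired fragment would apply level-scaled damage to the player and destroy the actor.
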(event OnComponentBeginOverlap(Collision)
  (params (OverlappedComponent :type Primitive%20Component%20Object%20Reference) (OtherActor :type Actor%20Object%20Reference) (OtherComp :type Primitive%20Component%20Object%20Reference) (OtherBodyIndex :type Integer) (bFromSweep :type Boolean) (SweepResult :type Hit%20Result%20Structure%20%28by%20ref%29)))

(event OnComponentHit(GeometryCollection)
  (params (HitComponent :type Primitive%20Component%20Object%20Reference) (OtherActor :type Actor%20Object%20Reference) (OtherComp :type Primitive%20Component%20Object%20Reference) (NormalImpulse :type Vector :default "0, 0, 0") (Hit :type Hit%20Result%20Structure%20%28by%20ref%29)))

(event EventTick
  (params (DeltaSeconds :type Float%20%28single-precision%29))
  (bind _returnvalue (* DeltaSeconds 1.5e+02))
  ;[1 1 1] Spin
  (Transformation|AddLocalRotation (Variables|Default|GetGeometryCollection) (Math|Rotator|MakeRotator _returnvalue _returnvalue _returnvalue) false false))

(event EventBeginPlay
  (Utilities|FlowControl|Delay 5.0)
  (Actor|DestroyActor))

(fn ConstructionScript)