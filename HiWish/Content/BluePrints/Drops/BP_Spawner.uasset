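; BP_Spawner continuously drops pickups and hazards from SpawnHeight at random Y positions.
; On BeginPlay it rolls chained percentage checks to spawn a pouch, diamond or gold, or otherwise a Bad2 with random spin.
; Each drop gets random projectile speeds capped by DropSpeed, then the graph loops back after a randomized delay around SpawnRate, with a short fallback range for low rates.
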(event EventBeginPlay
  (bind _returnvalue (Math|Random|RandomFloatinRange -1.2e+03 1.2e+03))
  (bind _returnvalue_2 (Math|Random|RandomIntegerinRange 0 99))
  (bind _dropspeed (Variables|Default|GetDropSpeed))
  (bind _spawnheight (Variables|Default|GetSpawnHeight))
  (bind _spawnrate (Variables|Default|GetSpawnRate))
  (bind _dropspeed_2 (Variables|Default|GetDropSpeed))
  (bind _dropspeed_3 (Variables|Default|GetDropSpeed))
  (bind _dropspeed_4 (Variables|Default|GetDropSpeed))
  (bind _returnvalue_3 (Math|Random|RandomFloatinRange 3e+02 _dropspeed_3))
  (bind _returnvalue_4 (Math|Random|RandomFloatinRange 3e+02 _dropspeed_2))
  (bind _returnvalue_5 (Math|Random|RandomFloatinRange 3e+02 _dropspeed_4))
  (bind _returnvalue_6 (Math|Random|RandomFloatinRange 3e+02 _dropspeed))
  (bind _returnvalue_7 (- _spawnrate 0.2))
  (if (<= (Math|Random|RandomIntegerinRange 0 99) (Variables|Default|GetGoodSpawnRate)) :!label _label
    (if (<= _returnvalue_2 (Variables|Default|GetPouchSpawnRate))
      (bind _returnvalue_8 (Game|SpawnActorfromClass "/Game/BluePrints/Drops/BP_Pouch.BP_Pouch_C" (Math|Transform|MakeTransform (Math|Vector|MakeVector 0.0 _returnvalue _spawnheight) "0, 0, 0" "1.000000,1.000000,1.000000") "Undefined" 0 0))
      (Variables|/Script/Engine.ProjectileMovementComponent|SetMaxSpeed (Variables|/Game/BluePrints/Drops/BP_Pouch.BP_Pouch_C|GetProjectileMovement _returnvalue_8) _returnvalue_4)
      (Variables|/Script/Engine.ProjectileMovementComponent|SetInitialSpeed (Variables|/Game/BluePrints/Drops/BP_Pouch.BP_Pouch_C|GetProjectileMovement _returnvalue_8) _returnvalue_4)
      (elif (<= _returnvalue_2 (Variables|Default|GetDiamondSpawnRate))
        (bind _returnvalue_9 (Game|SpawnActorfromClass "/Game/BluePrints/Drops/BP_Diamond.BP_Diamond_C" (Math|Transform|MakeTransform (Math|Vector|MakeVector 0.0 _returnvalue _spawnheight) "0, 0, 0" "4.000000,4.000000,4.000000") "Undefined" 0 0))
        (Variables|/Script/Engine.ProjectileMovementComponent|SetMaxSpeed (Variables|/Game/BluePrints/Drops/BP_Diamond.BP_Diamond_C|GetProjectileMovement _returnvalue_9) _returnvalue_5)
        (Variables|/Script/Engine.ProjectileMovementComponent|SetInitialSpeed (Variables|/Game/BluePrints/Drops/BP_Diamond.BP_Diamond_C|GetProjectileMovement _returnvalue_9) _returnvalue_5)
        (else
          (bind _returnvalue_10 (Game|SpawnActorfromClass "/Game/BluePrints/Drops/BP_Gold.BP_Gold_C" (Math|Transform|MakeTransform (Math|Vector|MakeVector 0.0 (Math|Random|RandomFloatinRange -1.2e+03 1.2e+03) (Variables|Default|GetSpawnHeight)) "0, 0, 0" "1.000000,1.000000,1.000000") "Undefined" 0 0))
          (Variables|/Script/Engine.ProjectileMovementComponent|SetMaxSpeed (Variables|/Game/BluePrints/Drops/BP_Gold.BP_Gold_C|GetProjectileMovement _returnvalue_10) _returnvalue_6)
          (Variables|/Script/Engine.ProjectileMovementComponent|SetInitialSpeed (Variables|/Game/BluePrints/Drops/BP_Gold.BP_Gold_C|GetProjectileMovement _returnvalue_10) _returnvalue_6))))
    (else
      (bind _returnvalue_11 (Game|SpawnActorfromClass "/Game/BluePrints/Drops/Bad2.Bad2_C" (Math|Transform|MakeTransform (Math|Vector|MakeVector 0.0 (Math|Random|RandomFloatinRange -1.2e+03 1.2e+03) (Variables|Default|GetSpawnHeight)) "0, 0, 0" "1.000000,1.000000,1.000000") "Undefined" 0 0))
      (Variables|/Script/Engine.ProjectileMovementComponent|SetMaxSpeed (Variables|/Game/BluePrints/Drops/Bad2.Bad2_C|GetProjectileMovement _returnvalue_11) _returnvalue_3)
      (Variables|/Script/Engine.ProjectileMovementComponent|SetInitialSpeed (Variables|/Game/BluePrints/Drops/Bad2.Bad2_C|GetProjectileMovement _returnvalue_11) _returnvalue_3)
      (Variables|/Script/Engine.RotatingMovementComponent|SetRotationRate (Variables|/Game/BluePrints/Drops/Bad2.Bad2_C|GetRotatingMovement _returnvalue_11) (Math|Rotator|MakeRotator (Math|Random|RandomFloatinRange -1e+02 1e+02) (Math|Random|RandomFloatinRange -1e+02 1e+02) (Math|Random|RandomFloatinRange -1e+02 1e+02)))))
  (if (<= _returnvalue_7 0.1)
    (Utilities|FlowControl|Delay (Math|Random|RandomFloatinRange 0.05 0.2))
    (goto _label)
    (else
      (Utilities|FlowControl|Delay (Math|Random|RandomFloatinRange _returnvalue_7 (+ _spawnrate 0.2)))
      (goto _label))))

(event EventTick
  (params (DeltaSeconds :type Float%20%28single-precision%29)))

(fn ConstructionScript)