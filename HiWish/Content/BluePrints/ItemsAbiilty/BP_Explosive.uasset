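; BP_Explosive is an ability actor whose expanding cube shatters Bad2 actors it touches.
; On BeginPlay, the Expand timeline pushes the cube along world Y and stretches its Z scale, lerping from current values each update so the change compounds.
; Overlapping a Bad2 enables physics on its Geometry Collection, disables its collision and plays a falling-stones sound.
; Money and score reward nodes are present but never run.
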(event OnComponentBeginOverlap(Cube)
  (params (OverlappedComponent :type Primitive%20Component%20Object%20Reference) (OtherActor :type Actor%20Object%20Reference) (OtherComp :type Primitive%20Component%20Object%20Reference) (OtherBodyIndex :type Integer) (bFromSweep :type Boolean) (SweepResult :type Hit%20Result%20Structure%20%28by%20ref%29))
  (bind _asbad_2 (Utilities|Casting|CastToBad2 OtherActor))
  (Physics|SetSimulatePhysics (Variables|/Game/BluePrints/Drops/Bad2.Bad2_C|GetGeometryCollection _asbad_2) true)
  (Collision|SetCollisionEnabled (Variables|/Game/BluePrints/Drops/Bad2.Bad2_C|GetCollision _asbad_2) "NoCollision")
  (Audio|PlaySound2D "/Game/Audio/08191_heavy_stones_falling-full.08191_heavy_stones_falling-full" 1.0 1.0 0.0 0 0))

(event EventBeginPlay
  (bind _cube (Variables|Default|GetCube))
  (bind _cube_2 (Variables|Default|GetCube))
  (bind _cube_3 (Variables|Default|GetCube))
  (bind _returnvalue (Transformation|GetWorldLocation _cube))
  (bind _returnvalue_2 (Transformation|GetWorldScale _cube_3))
  (bind _moving (Timeline|Expand PlayFromStart)
    (:Update
      (Transformation|SetWorldLocation _cube_2 (Math|Vector|MakeVector (.x _returnvalue) (Math|Float|Lerp (.y _returnvalue) (+ (.y _returnvalue) 8e+02) _moving) (.z _returnvalue)) false false)
      (Transformation|SetWorldScale3D _cube_2 (Math|Vector|MakeVector (.x _returnvalue_2) (.y _returnvalue_2) (Math|Float|Lerp (.z _returnvalue_2) (* (.z _returnvalue_2) 1e+01) _moving))))))

(event Collision|EventActorBeginOverlap
  (params (OtherActor :type Actor%20Object%20Reference)))

(event EventTick
  (params (DeltaSeconds :type Float%20%28single-precision%29)))

(fn ConstructionScript)